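; BP_Controller handles steering input for two local players by turning their player controllers.
; The Steer and SteerP2 axis events apply local yaw rotation to player controllers 0 and 1 respectively.
; Each turn scales the axis value by a shared TurnSpeed and world delta seconds for frame-rate independence.
; Rotation targets the controller actors directly, and BeginPlay, Tick and the construction script hold no logic.
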(event EventBeginPlay)

(event EventTick
  (params (DeltaSeconds :type Float%20%28single-precision%29)))

(event Input|AxisEvents|InputAxisSteer
  (params (AxisValue :type Float%20%28single-precision%29))
  (Transformation|AddActorLocalRotation (Game|GetPlayerController 0) (Math|Rotator|MakeRotator 0.0 0.0 (* AxisValue (Variables|Default|GetTurnSpeed) (Utilities|Time|GetWorldDeltaSeconds))) false false))

(event Input|AxisEvents|InputAxisSteerP2
  (params (AxisValue :type Float%20%28single-precision%29))
  (Transformation|AddActorLocalRotation (Game|GetPlayerController 1) (Math|Rotator|MakeRotator 0.0 0.0 (* AxisValue (Variables|Default|GetTurnSpeed) (Utilities|Time|GetWorldDeltaSeconds))) false false))

(fn ConstructionScript)