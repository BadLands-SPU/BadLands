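; BP_boat_Child is a boat variant, apparently derived from BP_boat, that adds steering for a second player.
; The SteerP2 input axis drives a local yaw rotation on the actor, scaled by TurnSpeed and frame delta time, without sweep.
; The construction script only calls the parent, the default events are disabled stubs, and a lookup of player controller 1 is left unused.
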(event EventBeginPlay
  (|CallParentFunction) ; This node is disabled and will not be called.\nDrag off pins to build functionality.
)

(event Collision|EventActorBeginOverlap
  (params (OtherActor :type Actor%20Object%20Reference))
  (|CallParentFunction OtherActor) ; This node is disabled and will not be called.\nDrag off pins to build functionality.
)

(event EventTick
  (params (DeltaSeconds :type Float%20%28single-precision%29))
  (|CallParentFunction DeltaSeconds) ; This node is disabled and will not be called.\nDrag off pins to build functionality.
)

(event Input|AxisEvents|InputAxisSteerP2
  (params (AxisValue :type Float%20%28single-precision%29))
  (Transformation|AddActorLocalRotation (Math|Rotator|MakeRotator 0.0 0.0 (* AxisValue (Variables|Default|GetTurnSpeed) (Utilities|Time|GetWorldDeltaSeconds))) false false))

(fn ConstructionScript
  (|CallParentFunction))